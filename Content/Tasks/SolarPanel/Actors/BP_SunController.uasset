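; BP_SunController is an actor in the solar panel task that rotates the level's sun and keeps its rotation in sync over the network.
; RotateSun runs only on authority, combining the sun's current rotation with the added rotation into the RepNotify variable SunRotation.
; OnRep_SunRotation applies that value to the sun and fires the OnSunRotated delegate, working around the lack of replication on directional lights.
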(fn ConstructionScript)

(fn RotateSun
  (params (AddRotation :type Rotator))
  ;[1 1 1] We can't just rotate directional light on the server, because replication is not available on lights, so this is workaround
  (Networking|SwitchHasAuthority
    (:Authority
      (Variables|Default|SetSunRotation (Math|Rotator|CombineRotators (Transformation|GetActorRotation (CallFunction|GetSun)) AddRotation)))))

(fn OnRepSunRotation
  (bind _sun (CallFunction|GetSun))
  (Utilities|IsValid _sun
    (:Is%20Valid
      (Transformation|SetActorRotation _sun (Variables|Default|GetSunRotation))
      (Default|CallOnSunRotatedDelegate))))