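; Solar panel actor that tracks and displays its efficiency based on how directly it faces the sun.
; The angle between the mesh's up vector and the reversed sun direction maps linearly to efficiency, reaching zero at 90 degrees or beyond.
; The server recalculates on construction, BeginPlay, sun-controller rotation events and panel rotation through RotateSolarPanel.
; The efficiency value's RepNotify refreshes the percentage text.
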(event Custom|OnSunRotatedDelegate
  (CallFunction|UpdateSolarPanelEfficiency))

(event EventBeginPlay
  (bind _suncontroller (CallFunction|GetSunController))
  (Networking|SwitchHasAuthority
    (:Authority
      (CallFunction|UpdateSolarPanelEfficiency)
      (Utilities|IsValid _suncontroller
        (:Is%20Valid
          (EventDispatchers|AssignOnSunRotatedDelegate _suncontroller (delegate Custom|OnSunRotatedDelegate)))))))

(fn ConstructionScript
  (CallFunction|UpdateSolarPanelEfficiency))

(fn GetAngleBetweenPanelandSun
  (bind _sun (CallFunction|GetSun))
  (bind _solarpanelmesh (Variables|Default|GetSolarPanelMesh))
  (bind _returnvalue (Math|Vector|GetUpVector _solarpanelmesh))
  (bind _returnvalue_2 (Transformation|GetActorForwardVector _sun))
  (bind _returnvalue_3 (* _returnvalue_2 -1.0))
  (Utilities|IsValid (CallFunction|GetSun)
    (:Is%20Valid
      (return (Class|KismetMathLibrary|DegAcos (/ (Math|Vector|DotProduct _returnvalue _returnvalue_3) (* (Math|Vector|VectorLength _returnvalue) (Math|Vector|VectorLength _returnvalue_3))))))
    (:Is%20Not%20Valid
      (return 0.0))))

(fn GetSolarPanelEfficiency
  (return (- 1.0 (/ (Math|Float|Clamp(Float) (CallFunction|GetAngleBetweenPanelandSun) 0.0 9e+01) 9e+01))))

(fn UpdateSolarPanelEfficiency
  (Networking|SwitchHasAuthority
    (:Authority
      (Variables|Default|SetSolarPanelEfficiency (CallFunction|GetSolarPanelEfficiency)))))

(fn UpdateSolarPanelEfficiencyText
  (Rendering|Components|TextRender|SetText (Variables|Default|GetEfficiencyText) (Utilities|Text|FormatText "Efficiency: {Efficiency}%" (Utilities|Text|ToText(Float) (* (Variables|Default|GetSolarPanelEfficiency) 1e+02) "HalfToEven" false true 1 324 0 2))))

(fn RotateSolarPanel
  (params (AddRotation :type Rotator))
  (Networking|SwitchHasAuthority
    (:Authority
      (Class|Actor|AddActorWorldRotation AddRotation)
      (CallFunction|UpdateSolarPanelEfficiency))))

(fn OnRepSolarPanelEfficiency
  (CallFunction|UpdateSolarPanelEfficiencyText))