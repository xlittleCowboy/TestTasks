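; Debug variant of a solar panel that spins to random orientations, apparently for testing rotation and efficiency.
; On BeginPlay, only the authority starts a looping timer on TimeToRandomlyRotate, presumably bound to RandomlyRotateSolarPanel, which passes a random rotator to RotateSolarPanel.
; The construction script places EfficiencyText above the actor along world up.
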(event EventBeginPlay
  (|CallParentFunction)
  (Networking|SwitchHasAuthority
    (:Authority
      (Utilities|Time|SetTimerbyEvent (EventDispatchers|CreateEvent :!event RandomlyRotateSolarPanel) (Variables|DebugSolarPanelSettings|GetTimeToRandomlyRotate) true))))

(event Collision|EventActorBeginOverlap
  (params (OtherActor :type Actor%20Object%20Reference)))

(event EventTick
  (params (DeltaSeconds :type Float%20%28single-precision%29)))

(fn ConstructionScript
  (|CallParentFunction)
  (Transformation|SetWorldLocation (Variables|Default|GetEfficiencyText) (+ (Transformation|GetActorLocation) (* "0.000000,0.000000,1.000000" 1e+02)) false false))

(fn RandomlyRotateSolarPanel
  (CallFunction|RotateSolarPanel (Math|Random|RandomRotator true)))