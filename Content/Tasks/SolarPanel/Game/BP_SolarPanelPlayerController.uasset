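; Player controller for the solar panel task that lets the player rotate the sun one axis at a time.
; On BeginPlay it adds input mapping contexts; inputs call server events that cycle the rotation axis or rotate by input times sensitivity.
; Rotation goes through the sun controller rather than the directional light so subscribed solar panels can update their efficiency.
; The replicated axis's OnRep broadcasts the new mode through a delegate.
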(event Custom|SERVER_ChangeSunRotation
  (params (Amount :type Float%20%28double-precision%29))
  ;[1 1 1] Sun Control Server Events
  (CallFunction|ChangeSunRotation Amount))

(event Custom|SERVER_ChangeSunRotationMode
  ;[1 1 1] Sun Control Server Events
  (CallFunction|ChangeSunRotationMode))

(event Custom|SERVER_ChangeSunRotationSensitivity
  (params (Sensitivity :type Float%20%28double-precision%29))
  ;[1 1 1] Sun Control Server Events
  (Variables|Settings|SetSunRotationSensitivity Sensitivity))

(event Input|EnhancedActionEvents|EnhancedInputActionIA_ChangeSunRotationMode
  (params (ActionValue :type Boolean) (ElapsedSeconds :type Float%20%28double-precision%29) (TriggeredSeconds :type Float%20%28double-precision%29) (InputAction :type Input%20Action%20Object%20Reference :default "/Game/Tasks/SolarPanel/Input/IA_ChangeSunRotationMode.IA_ChangeSunRotationMode"))
  ;[1 1 1] Sun Control Inputs
  (CallFunction|SERVERChangeSunRotationMode))

(event Input|EnhancedActionEvents|EnhancedInputActionIA_ChangeSunRotation
  (params (ActionValue :type Float%20%28double-precision%29) (ElapsedSeconds :type Float%20%28double-precision%29) (TriggeredSeconds :type Float%20%28double-precision%29) (InputAction :type Input%20Action%20Object%20Reference :default "/Game/Tasks/SolarPanel/Input/IA_ChangeSunRotation.IA_ChangeSunRotation"))
  ;[1 1 1] Sun Control Inputs
  (CallFunction|SERVERChangeSunRotation ActionValue))

(event EventBeginPlay
  (bind _returnvalue (PlayerController|LocalPlayerSubsystems|GetEnhancedInputLocalPlayerSubsystem))
  ;[1 0 0] Begin Play
  ;[1 1 1] Add Mapping Contexts
  (Utilities|IsValid _returnvalue
    (:Is%20Valid
      (for _array_element (Variables|Input|GetStartMappingContexts)
        (Input|AddMappingContext _returnvalue _array_element 0 "(bIgnoreAllPressedKeysUntilRelease=True,bForceImmediately=False,bNotifyUserSettings=False)")))))

(fn ConstructionScript)

(fn ChangeSunRotationMode
  (if (Utilities|Operators|EqualEqual (Variables|Settings|GetSunRotator) "0.000000,0.000000,1.000000" 0.1)
    (Variables|Settings|SetSunRotator "1.000000,0.000000,0.000000")
    (elif (Utilities|Operators|EqualEqual (Variables|Settings|GetSunRotator) "1.000000,0.000000,0.000000" 0.1)
      (Variables|Settings|SetSunRotator "0.000000,1.000000,0.000000")
      (else
        (Variables|Settings|SetSunRotator "0.000000,0.000000,1.000000")))))

(fn ChangeSunRotation
  (params (Amount :type Float%20%28double-precision%29))
  (bind _suncontroller (CallFunction|GetSunController))
  (Utilities|IsValid _suncontroller
    (:Is%20Valid
      (Default|RotateSun _suncontroller (* (Variables|Settings|GetSunRotator) (* Amount (Variables|Settings|GetSunRotationSensitivity)))) ; We don't rotate directional light straightforward, because solar panels need to know when sun is rotated.\nWhen we rotate directional light with BP_SunController, OnSunRotatedDelegate fires and all solar panels,\nthat are subscribed to this event, can update their efficiency.
    )))

(fn OnRepSunRotator
  (if (Utilities|Operators|EqualEqual (Variables|Settings|GetSunRotator) "0.000000,0.000000,1.000000" 0.1)
    (Default|CallOnSunRotationModeChangedDelegate "X")
    (elif (Utilities|Operators|EqualEqual (Variables|Settings|GetSunRotator) "1.000000,0.000000,0.000000" 0.1)
      (Default|CallOnSunRotationModeChangedDelegate "Y")
      (else
        (Default|CallOnSunRotationModeChangedDelegate "Z")))))