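; Player controller that lets the player command all drones by aiming with the camera.
; On BeginPlay it adds its starting Enhanced Input mapping contexts.
; Two input actions line-trace from the camera, with debug drawing, to pick either a hit location or a hit actor.
; Server events then pass that target to every FlyingAIController found in the world, updating each drone's fly-to destination.
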(event Custom|SERVER_SendAllDronesToLocation
  (params (Location :type Vector))
  ;[1 1 1] Drone control
  (CallFunction|SendAllDronestoLocation Location))

(event Custom|SERVER_SendAllDronesToActor
  (params (Actor :type Actor%20Object%20Reference))
  ;[1 1 1] Drone control
  (CallFunction|SendAllDronestoActor Actor))

(event Input|EnhancedActionEvents|EnhancedInputActionIA_SetDroneTargetLocation
  (params (ActionValue :type Boolean) (ElapsedSeconds :type Float%20%28double-precision%29) (TriggeredSeconds :type Float%20%28double-precision%29) (InputAction :type Input%20Action%20Object%20Reference :default "/Game/Tasks/Drone/Input/IA_SetDroneTargetLocation.IA_SetDroneTargetLocation"))
  ;[1 1 1] Drone control
  (bind (_hitsomething _outhit) (CallFunction|LineTracefromCamera self (Variables|Default|GetSendDroneDistance) "TraceTypeQuery1" "ForDuration" "(R=1.000000,G=0.000000,B=0.000000,A=1.000000)"))
  (if _hitsomething
    (CallFunction|SERVERSendAllDronestoLocation (.Location (Collision|BreakHitResult _outhit)))))

(event Input|EnhancedActionEvents|EnhancedInputActionIA_SetDroneTargetActor
  (params (ActionValue :type Boolean) (ElapsedSeconds :type Float%20%28double-precision%29) (TriggeredSeconds :type Float%20%28double-precision%29) (InputAction :type Input%20Action%20Object%20Reference :default "/Game/Tasks/Drone/Input/IA_SetDroneTargetActor.IA_SetDroneTargetActor"))
  ;[1 1 1] Drone control
  (bind (_hitsomething _outhit) (CallFunction|LineTracefromCamera self (Variables|Default|GetSendDroneDistance) "TraceTypeQuery1" "ForDuration" "(R=0.000000,G=0.000000,B=0.984000,A=1.000000)"))
  (if _hitsomething
    (CallFunction|SERVERSendAllDronestoActor (.HitActor (Collision|BreakHitResult _outhit)))))

(event EventBeginPlay
  (bind _returnvalue (PlayerController|LocalPlayerSubsystems|GetEnhancedInputLocalPlayerSubsystem))
  ;[1 0 0] Begin Play
  ;[1 1 1] Add Mapping Contexts
  (Utilities|IsValid _returnvalue
    (:Is%20Valid
      (for _array_element (Variables|Default|GetStartMappingContexts)
        (Input|AddMappingContext _returnvalue _array_element 0 "(bIgnoreAllPressedKeysUntilRelease=True,bForceImmediately=False,bNotifyUserSettings=False)")))))

(fn ConstructionScript)

(fn SendAllDronestoLocation
  (params (Location :type Vector))
  (bind _outactors (Actor|GetAllActorsOfClass "/Script/TestTasks.FlyingAIController"))
  (for _array_element _outactors
    (Class|FlyingAIController|UpdateFlytoLocation _array_element Location)))

(fn SendAllDronestoActor
  (params (Actor :type Actor%20Object%20Reference))
  (bind _outactors (Actor|GetAllActorsOfClass "/Script/TestTasks.FlyingAIController"))
  (for _array_element _outactors
    (Class|FlyingAIController|UpdateFlytoActor _array_element Actor)))