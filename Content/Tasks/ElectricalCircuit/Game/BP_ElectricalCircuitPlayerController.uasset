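; Player controller for the electrical circuit task, handling interaction and the linking of electrical devices.
; On begin play it adds its starting input mapping contexts; the interact input line-traces from the camera and sends an interact message to the hit actor.
; The connect input stores the first traced device, then connects it both ways to the second, undoing the first link if the reverse fails, with colored on-screen status messages.
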(event Input|EnhancedActionEvents|EnhancedInputActionIA_Interact
  (params (ActionValue :type Boolean) (ElapsedSeconds :type Float%20%28double-precision%29) (TriggeredSeconds :type Float%20%28double-precision%29) (InputAction :type Input%20Action%20Object%20Reference :default "/Game/Tasks/ElectricalCircuit/Input/IA_Interact.IA_Interact"))
  ;[1 1 1] Interaction
  (bind (_hitsomething _outhit) (CallFunction|LineTracefromCamera self (Variables|Default|GetInteractionDistance) "TraceTypeQuery3" "None" "(R=1.000000,G=0.000000,B=0.000000,A=1.000000)"))
  (if _hitsomething
    (Class|BPIInteraction|Interact(Message) (.HitActor (Collision|BreakHitResult _outhit)) (Pawn|GetControlledPawn) self)))

(event Input|EnhancedActionEvents|EnhancedInputActionIA_ConnectElectricalDevices
  (params (ActionValue :type Boolean) (ElapsedSeconds :type Float%20%28double-precision%29) (TriggeredSeconds :type Float%20%28double-precision%29) (InputAction :type Input%20Action%20Object%20Reference :default "/Game/Tasks/ElectricalCircuit/Input/IA_ConnectElectricalDevices.IA_ConnectElectricalDevices"))
  ;[1 1 1] Devices Connection
  (bind (_hitsomething _outhit) (CallFunction|LineTracefromCamera self (Variables|Default|GetInteractionDistance) "TraceTypeQuery3" "None" "(R=1.000000,G=0.000000,B=0.000000,A=1.000000)"))
  (if _hitsomething
    (Utilities|IsValid (Actor|GetComponentbyClass (.HitActor (Collision|BreakHitResult _outhit)) "/Script/TestTasks.ElectricalDeviceComponent")
      (:Is%20Valid
        (Utilities|IsValid (Variables|Default|GetConnectingDevice)
          (:Is%20Valid
            (bind _success (Class|BPIElectricalDevice|ConnectDevice(Message) (Variables|Default|GetConnectingDevice) (.HitActor (Collision|BreakHitResult _outhit)) self))
            (if _success
              (bind _success_2 (Class|BPIElectricalDevice|ConnectDevice(Message) (.HitActor (Collision|BreakHitResult _outhit)) (Variables|Default|GetConnectingDevice) self))
              (if _success_2
                (Development|PrintString (Utilities|String|ToString(Text) (Utilities|Text|FormatText "Successfully connected {Device1} to {Device2}" (Variables|Default|GetConnectingDevice) (.HitActor (Collision|BreakHitResult _outhit)))) true true "(R=0.000000,G=1.000000,B=0.000000,A=1.000000)" 1e+01 "1")
                (Variables|Default|SetConnectingDevice 0)
                (else
                  (Class|BPIElectricalDevice|UnconnectDevice(Message) (Variables|Default|GetConnectingDevice) (.HitActor (Collision|BreakHitResult _outhit)) self)
                  (Development|PrintString (Utilities|String|ToString(Text) (Utilities|Text|FormatText "Failed to connect {Device1} to {Device2}" (Variables|Default|GetConnectingDevice) (.HitActor (Collision|BreakHitResult _outhit)))) true true "(R=1.000000,G=0.000000,B=0.000000,A=1.000000)" 1e+01 "1" :!label _label)
                  (Variables|Default|SetConnectingDevice 0)))
              (else
                (goto _label))))
          (:Is%20Not%20Valid
            (Variables|Default|SetConnectingDevice (.HitActor (Collision|BreakHitResult _outhit)))
            (Development|PrintString (Utilities|String|ToString(Text) (Utilities|Text|FormatText "Connecting {Device1} to ..." (Variables|Default|GetConnectingDevice))) true true "(R=1.000000,G=1.000000,B=0.000000,A=1.000000)" 99999999.0 "1")))))))

(event EventBeginPlay
  (bind _returnvalue (PlayerController|LocalPlayerSubsystems|GetEnhancedInputLocalPlayerSubsystem))
  ;[1 0 0] Begin Play
  ;[1 1 1] Add Mapping Contexts
  (Utilities|IsValid _returnvalue
    (:Is%20Valid
      (for _array_element (Variables|Default|GetStartMappingContexts)
        (Input|AddMappingContext _returnvalue _array_element 0 "(bIgnoreAllPressedKeysUntilRelease=True,bForceImmediately=False,bNotifyUserSettings=False)")))))

(fn ConstructionScript)