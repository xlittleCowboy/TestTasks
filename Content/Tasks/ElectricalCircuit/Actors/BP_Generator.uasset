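; Generator actor for the electrical circuit task that lets switch devices be connected to it and disconnected from it.
; ConnectDevice and UnconnectDevice fetch the BP_EDD_Generator definition from its ElectricalDevice and forward the device to ConnectSwitch or UnconnectSwitch.
; Each call passes the generator as the cause along with the instigator, and returns the definition's result.
; The actor holds no other logic, as its event graph and construction script are empty.
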(event EventBeginPlay)

(event Collision|EventActorBeginOverlap
  (params (OtherActor :type Actor%20Object%20Reference)))

(event EventTick
  (params (DeltaSeconds :type Float%20%28single-precision%29)))

(fn ConstructionScript)

(fn ConnectDevice
  (params (DeviceToConnect :type Actor%20Object%20Reference) (Instigated :type Controller%20Object%20Reference))
  (bind _success (Default|ConnectSwitch (Class|ElectricalDeviceComponent|GetElectricalDeviceDefinitionCasted (Variables|Default|GetElectricalDevice) "/Game/Tasks/ElectricalCircuit/Devices/BP_EDD_Generator.BP_EDD_Generator_C") DeviceToConnect self Instigated))
  (return _success))

(fn UnconnectDevice
  (params (DeviceToUnconnect :type Actor%20Object%20Reference) (Instigated :type Controller%20Object%20Reference))
  (bind _success (Default|UnconnectSwitch (Class|ElectricalDeviceComponent|GetElectricalDeviceDefinitionCasted (Variables|Default|GetElectricalDevice) "/Game/Tasks/ElectricalCircuit/Devices/BP_EDD_Generator.BP_EDD_Generator_C") DeviceToUnconnect self Instigated))
  (return _success))