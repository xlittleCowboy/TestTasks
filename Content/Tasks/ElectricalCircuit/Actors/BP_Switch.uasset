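; BP_Switch is an interactable electrical circuit switch that toggles the devices connected to it.
; Toggling plays the skeletal mesh animation forward or in reverse based on TurnedOn, then calls TurnAllConnectedDevices on the ElectricalDevice component's BP_EDD_Switch definition.
; Connect and unconnect functions forward to that same definition.
; A switch set on in the editor resets TurnedOn at BeginPlay and runs the normal toggle.
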(event EventInteract
  (params (Interactor :type Actor%20Object%20Reference) (InteractorController :type Controller%20Object%20Reference))
  ;[1 1 1] Turn switch on/off
  (CallFunction|TurnSwitch InteractorController))

(event EventBeginPlay
  (bind _electricaldevice (Variables|Default|GetElectricalDevice))
  (bind _returnvalue (Class|ElectricalDeviceComponent|GetElectricalDeviceDefinitionCasted _electricaldevice "/Game/Tasks/ElectricalCircuit/Devices/BP_EDD_Switch.BP_EDD_Switch_C"))
  ;[1 0 0] Begin Play
  ;[1 1 1] If TurnedOn variable was set to true in editor, then we turn this switch on
  (if (Variables|/Game/Tasks/ElectricalCircuit/Devices/BP_EDD_Switch.BP_EDD_Switch_C|GetTurnedOn _returnvalue)
    (Variables|/Game/Tasks/ElectricalCircuit/Devices/BP_EDD_Switch.BP_EDD_Switch_C|SetTurnedOn _returnvalue false)
    (CallFunction|TurnSwitch)))

(fn ConstructionScript)

(fn PlayTurnAnimation
  (if (Variables|/Game/Tasks/ElectricalCircuit/Devices/BP_EDD_Switch.BP_EDD_Switch_C|GetTurnedOn (Class|ElectricalDeviceComponent|GetElectricalDeviceDefinitionCasted (Variables|Default|GetElectricalDevice) "/Game/Tasks/ElectricalCircuit/Devices/BP_EDD_Switch.BP_EDD_Switch_C"))
    (Components|Timeline|SetPlayRate (Variables|Default|GetSkeletalMesh) -4.0)
    (else
      (Components|Timeline|SetPlayRate (Variables|Default|GetSkeletalMesh) 4.0)))
  (Audio|Components|Audio|Play (Variables|Default|GetSkeletalMesh) false))

(fn TurnSwitch
  (params (InstigatedBy :type Controller%20Object%20Reference))
  (CallFunction|PlayTurnAnimation)
  (Default|TurnAllConnectedDevices (Class|ElectricalDeviceComponent|GetElectricalDeviceDefinitionCasted (Variables|Default|GetElectricalDevice) "/Game/Tasks/ElectricalCircuit/Devices/BP_EDD_Switch.BP_EDD_Switch_C") self InstigatedBy))

(fn ConnectDevice
  (params (DeviceToConnect :type Actor%20Object%20Reference) (Instigated :type Controller%20Object%20Reference))
  (bind _success (Default|ConnectDeviceorGenerator (Class|ElectricalDeviceComponent|GetElectricalDeviceDefinitionCasted (Variables|Default|GetElectricalDevice) "/Game/Tasks/ElectricalCircuit/Devices/BP_EDD_Switch.BP_EDD_Switch_C") DeviceToConnect self Instigated))
  (return _success))

(fn UnconnectDevice
  (params (DeviceToUnconnect :type Actor%20Object%20Reference) (Instigated :type Controller%20Object%20Reference))
  (bind _success (Default|UnconnectDeviceorGenerator (Class|ElectricalDeviceComponent|GetElectricalDeviceDefinitionCasted (Variables|Default|GetElectricalDevice) "/Game/Tasks/ElectricalCircuit/Devices/BP_EDD_Switch.BP_EDD_Switch_C") DeviceToUnconnect self Instigated))
  (return _success))