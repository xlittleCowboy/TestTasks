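; BP_EDD_Consumer is the electrical device definition for a power consumer in the electrical circuit task.
; It exposes its power consumption and holds a reference to a single connected switch actor.
; Connecting succeeds only when no valid switch is already linked and the actor carries a BP_EDD_Switch definition.
; Disconnecting simply clears the reference and always reports success.
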(fn ConnectSwitch
  (params (SwitchToConnect :type Actor%20Object%20Reference) (CausedBy :type Actor%20Object%20Reference) (InstigatedBy :type Controller%20Object%20Reference))
  (Utilities|IsValid (Variables|Default|GetConnectedSwitch)
    (:Is%20Valid
      (return false))
    (:Is%20Not%20Valid
      (Utilities|IsValid (Class|ElectricalDeviceComponent|GetElectricalDeviceDefinitionfromActor SwitchToConnect "/Game/Tasks/ElectricalCircuit/Devices/BP_EDD_Switch.BP_EDD_Switch_C")
        (:Is%20Valid
          (Consumer|UnconnectSwitch CausedBy InstigatedBy)
          (Variables|Default|SetConnectedSwitch SwitchToConnect)
          (return true))
        (:Is%20Not%20Valid
          (return false))))))

(fn UnconnectSwitch
  (params (CausedBy :type Actor%20Object%20Reference) (InstigatedBy :type Controller%20Object%20Reference))
  (Variables|Default|SetConnectedSwitch 0)
  (return true))

(fn GetPowerConsumption
  (return (Variables|Consumer|GetPowerConsumption)))