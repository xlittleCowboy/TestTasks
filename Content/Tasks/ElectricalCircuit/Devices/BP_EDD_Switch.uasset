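; Switch device definition for the electrical circuit task, linking a set of consumer devices to a single generator.
; Toggling it flips TurnedOn and asks the generator to turn all connected devices on or off.
; Connecting while on powers devices through the generator, and disconnecting tells the generator to turn them off.
; Combined connect and disconnect functions try the actor as a device first, then as a generator.
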(fn TurnAllConnectedDevices
  (params (CausedBy :type Actor%20Object%20Reference) (InstigatedBy :type Controller%20Object%20Reference))
  (if (Variables|Switch|GetTurnedOn)
    (Variables|Switch|SetTurnedOn false)
    (bind _connectedgenerator (Variables|Switch|GetConnectedGenerator)
      (:then
        (Utilities|IsValid (Class|ElectricalDeviceComponent|GetElectricalDeviceDefinitionfromActor _connectedgenerator "/Game/Tasks/ElectricalCircuit/Devices/BP_EDD_Generator.BP_EDD_Generator_C")
          (:Is%20Valid
            (Default|TurnOffDevices (Class|ElectricalDeviceComponent|GetElectricalDeviceDefinitionfromActor _connectedgenerator "/Game/Tasks/ElectricalCircuit/Devices/BP_EDD_Generator.BP_EDD_Generator_C") (Variables|Switch|GetConnectedDevices) CausedBy InstigatedBy))))
      (:else))
    (else
      (Variables|Switch|SetTurnedOn true)
      (bind _connectedgenerator_2 (Variables|Switch|GetConnectedGenerator)
        (:then
          (Utilities|IsValid (Class|ElectricalDeviceComponent|GetElectricalDeviceDefinitionfromActor _connectedgenerator_2 "/Game/Tasks/ElectricalCircuit/Devices/BP_EDD_Generator.BP_EDD_Generator_C")
            (:Is%20Valid
              (Default|TurnonDevices (Class|ElectricalDeviceComponent|GetElectricalDeviceDefinitionfromActor _connectedgenerator "/Game/Tasks/ElectricalCircuit/Devices/BP_EDD_Generator.BP_EDD_Generator_C") (Variables|Switch|GetConnectedDevices) CausedBy InstigatedBy))))
        (:else)))))

(fn ConnectDevice
  (params (DeviceToConnect :type Actor%20Object%20Reference) (CausedBy :type Actor%20Object%20Reference) (InstigatedBy :type Controller%20Object%20Reference))
  (Utilities|IsValid (Class|ElectricalDeviceComponent|GetElectricalDeviceDefinitionfromActor DeviceToConnect "/Game/Tasks/ElectricalCircuit/Devices/BP_EDD_Consumer.BP_EDD_Consumer_C")
    (:Is%20Valid
      (bind _returnvalue (Utilities|Array|AddUnique (Variables|Switch|GetConnectedDevices) DeviceToConnect))
      (if (>= _returnvalue 0)
        (if (Variables|Switch|GetTurnedOn)
          (bind _connectedgenerator (Variables|Switch|GetConnectedGenerator)
            (:then
              (Default|TurnonDevice (Class|ElectricalDeviceComponent|GetElectricalDeviceDefinitionfromActor _connectedgenerator "/Game/Tasks/ElectricalCircuit/Devices/BP_EDD_Generator.BP_EDD_Generator_C") DeviceToConnect CausedBy InstigatedBy)
              (return true))
            (:else
              (return true)))
          (else
            (return true)))
        (else
          (return false))))))

(fn UnconnectDevice
  (params (DeviceToUnconnect :type Actor%20Object%20Reference) (CausedBy :type Actor%20Object%20Reference) (InstigatedBy :type Controller%20Object%20Reference))
  (bind _returnvalue (Utilities|Array|RemoveItem (Variables|Switch|GetConnectedDevices) DeviceToUnconnect))
  (if _returnvalue
    (bind _connectedgenerator (Variables|Switch|GetConnectedGenerator)
      (:then
        (Default|TurnOffDevice (Class|ElectricalDeviceComponent|GetElectricalDeviceDefinitionfromActor _connectedgenerator "/Game/Tasks/ElectricalCircuit/Devices/BP_EDD_Generator.BP_EDD_Generator_C") DeviceToUnconnect CausedBy InstigatedBy)
        (return true))
      (:else
        (return true)))
    (else
      (return false))))

(fn ConnectGenerator
  (params (GeneratorToConnect :type Actor%20Object%20Reference) (CausedBy :type Actor%20Object%20Reference) (InstigatedBy :type Controller%20Object%20Reference))
  (Utilities|IsValid (Class|ElectricalDeviceComponent|GetElectricalDeviceDefinitionfromActor GeneratorToConnect "/Game/Tasks/ElectricalCircuit/Devices/BP_EDD_Generator.BP_EDD_Generator_C")
    (:Is%20Valid
      (if (!= GeneratorToConnect (Variables|Switch|GetConnectedGenerator))
        (Variables|Switch|SetConnectedGenerator GeneratorToConnect)
        (if (Variables|Switch|GetTurnedOn)
          (Default|TurnonDevices (Class|ElectricalDeviceComponent|GetElectricalDeviceDefinitionfromActor (Variables|Switch|GetConnectedGenerator) "/Game/Tasks/ElectricalCircuit/Devices/BP_EDD_Generator.BP_EDD_Generator_C") (Variables|Switch|GetConnectedDevices) CausedBy InstigatedBy)
          (return true)
          (else
            (return true)))
        (else
          (return false))))
    (:Is%20Not%20Valid
      (return false))))

(fn UnconnectGenerator
  (params (GeneratorToUnconnect :type Actor%20Object%20Reference) (CausedBy :type Actor%20Object%20Reference) (InstigatedBy :type Controller%20Object%20Reference))
  (if (== GeneratorToUnconnect (Variables|Switch|GetConnectedGenerator))
    (Default|TurnOffDevices (Class|ElectricalDeviceComponent|GetElectricalDeviceDefinitionfromActor (Variables|Switch|GetConnectedGenerator) "/Game/Tasks/ElectricalCircuit/Devices/BP_EDD_Generator.BP_EDD_Generator_C") (Variables|Switch|GetConnectedDevices) CausedBy InstigatedBy)
    (Variables|Switch|SetConnectedGenerator 0)
    (return true)
    (else
      (return false))))

(fn ConnectDeviceorGenerator
  (params (DeviceToConnect :type Actor%20Object%20Reference) (CausedBy :type Actor%20Object%20Reference) (InstigatedBy :type Controller%20Object%20Reference))
  (bind _success (Switch|ConnectDevice DeviceToConnect CausedBy InstigatedBy))
  (if _success
    (return true)
    (else
      (bind _success_2 (Switch|ConnectGenerator DeviceToConnect CausedBy InstigatedBy))
      (return _success_2))))

(fn UnconnectDeviceorGenerator
  (params (DeviceToUnconnect :type Actor%20Object%20Reference) (CausedBy :type Actor%20Object%20Reference) (InstigatedBy :type Controller%20Object%20Reference))
  (bind _success (Switch|UnconnectDevice DeviceToUnconnect CausedBy InstigatedBy))
  (if _success
    (return true)
    (else
      (bind _success_2 (Switch|UnconnectGenerator DeviceToUnconnect CausedBy InstigatedBy))
      (return _success_2))))