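; Generator device definition for the electrical circuit task that switches consumer devices on and off within a maximum power budget.
; TurnOnDevice reads each actor's BP_EDD_Consumer draw, then either powers it and records the draw or adds it to a waiting collection if over budget.
; TurnOffDevice frees the recorded draw and drops the device from waiting.
; After a batch turn-off, TurnOffDevices retries waiting devices with the freed capacity.
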(fn TurnonDevices
  (params (Devices :type Array%20of%20Actor%20Object%20References) (CausedBy :type Actor%20Object%20Reference) (InstigatedBy :type Controller%20Object%20Reference))
  (for _array_element Devices
    (Generator|TurnonDevice _array_element CausedBy InstigatedBy)))

(fn TurnOffDevices
  (params (Devices :type Array%20of%20Actor%20Object%20References) (CausedBy :type Actor%20Object%20Reference) (InstigatedBy :type Controller%20Object%20Reference))
  (for _array_element Devices
    (Generator|TurnOffDevice _array_element CausedBy InstigatedBy))
  (Generator|TurnonDevices (Variables|Generator|GetDevicesThatWantConsumePower) 0 InstigatedBy))

(fn TurnonDevice
  (params (DeviceToTurnOn :type Actor%20Object%20Reference) (CausedBy :type Actor%20Object%20Reference) (InstigatedBy :type Controller%20Object%20Reference))
  (bind _returnvalue (Class|ElectricalDeviceComponent|GetElectricalDeviceDefinitionfromActor DeviceToTurnOn "/Game/Tasks/ElectricalCircuit/Devices/BP_EDD_Consumer.BP_EDD_Consumer_C"))
  (bind _consumption (Default|GetPowerConsumption _returnvalue))
  (if (not (.ReturnValue (Utilities|Map|Find (Variables|Generator|GetPowerConsumingDevices) DeviceToTurnOn)))
    (Utilities|IsValid _returnvalue
      (:Is%20Valid
        (if (<= (+ _consumption (Variables|Generator|GetTotalPowerConsumption)) (Variables|Generator|GetMaximumPowerConsumption))
          (Variables|Generator|SetTotalPowerConsumption (+ _consumption (Variables|Generator|GetTotalPowerConsumption)))
          (Utilities|Map|Add (Variables|Generator|GetPowerConsumingDevices) DeviceToTurnOn _consumption)
          (Class|BPIElectricalDevice|Turnon(Message) DeviceToTurnOn CausedBy InstigatedBy)
          (Utilities|Array|RemoveItem (Variables|Generator|GetDevicesThatWantConsumePower) DeviceToTurnOn)
          (else
            (Utilities|Array|Add (Variables|Generator|GetDevicesThatWantConsumePower) DeviceToTurnOn)))))))

(fn TurnOffDevice
  (params (DeviceToTurnOff :type Actor%20Object%20Reference) (CausedBy :type Actor%20Object%20Reference) (InstigatedBy :type Controller%20Object%20Reference))
  (bind _powerconsumingdevices (Variables|Generator|GetPowerConsumingDevices))
  (bind (_value _returnvalue) (Utilities|Map|Find _powerconsumingdevices DeviceToTurnOff))
  (if _returnvalue
    (Variables|Generator|SetTotalPowerConsumption (- (Variables|Generator|GetTotalPowerConsumption) _value))
    (Class|BPIElectricalDevice|TurnOff(Message) DeviceToTurnOff CausedBy InstigatedBy)
    (Utilities|Map|Remove (Variables|Generator|GetPowerConsumingDevices) DeviceToTurnOff)
    (Utilities|Array|RemoveItem (Variables|Generator|GetDevicesThatWantConsumePower) DeviceToTurnOff)
    (else
      (Utilities|Array|RemoveItem (Variables|Generator|GetDevicesThatWantConsumePower) DeviceToTurnOff))))